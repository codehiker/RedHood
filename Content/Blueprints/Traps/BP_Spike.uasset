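; Spike trap for a 2D Paper2D game that primes on the first overlap, then damages characters that touch it.
; The first overlap plays a one-shot flipbook and trigger sound; overlaps during priming deal no damage.
; When the flipbook finishes, it becomes primed, shows the spike sprite and manually damages an overlapping BP_RedHood.
; Later overlaps call GetHit on any BP_CharacterBase and switch to the hit sprite.
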(event `self.ReceiveActorBeginOverlap`
  (params (OtherActor :type "Actor Object Reference"))
  ;[0.2703 0.3551 0.849] Decide whether to prime the trap or damage the player. The only time a trap will not damage the player is if the trap is priming, which only happens once.
  (if (or (`self.Primed`) (`self.Priming`))
    (if (`self.Primed`)
      (`self.DamageTarget` OtherActor)
      (`PaperSpriteComponent.SetSprite` (`self.RenderComponent`) (`self.Spike_Hit`)))
    (else
      (`self.TriggerTrap`))))

(event `self.PaperFlipbook.OnFinishedPlaying`
  (bind _output (`|GetArrayItem` (`PrimitiveComponent.GetOverlappingActors` (`self.Box`) "/Game/Blueprints/Characters/RedHood/BP_RedHood.BP_RedHood_C")))
  ;[0.2703 0.3551 0.849] When the trap animation completes, we want to enable damage. The overlap event has already been triggered, so we have to manually apply damage the first time.
  (`PaperSpriteComponent.SetSprite` (`self.RenderComponent`) (`self.Spike_Visible`))
  (`SceneComponent.SetVisibility` (`self.PaperFlipbook`) false false)
  (set `self.Priming` false)
  (set `self.Primed` true)
  (`/Engine/EditorBlueprintResources/StandardMacros.IsValid` _output
    (:`Is Valid`
      (`self.DamageTarget` _output)
      (`PaperSpriteComponent.SetSprite` (`self.RenderComponent`) (`self.Spike_Hit`)))))

(fn `DamageTarget`
  (params (CharacterToDamage :type "Actor Object Reference"))
  (bind _asbp_character_base (cast `/Game/Blueprints/Characters/BP_CharacterBase` CharacterToDamage))
  (`/Game/Blueprints/Characters/BP_CharacterBase.Get Hit` _asbp_character_base (`self.Damage`)))

(fn `TriggerTrap`
  (set `self.Priming` true)
  (`SceneComponent.SetVisibility` (`self.PaperFlipbook`) true false)
  (`PaperFlipbookComponent.SetLooping` (`self.PaperFlipbook`) false)
  (`PaperFlipbookComponent.PlayFromStart` (`self.PaperFlipbook`))
  (`GameplayStatics.PlaySound2D` (`self.TrapTriggerSound`) 1.0 1.0 0.0 null null))

(fn `UserConstructionScript`)