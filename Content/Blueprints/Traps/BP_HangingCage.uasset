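; Hanging cage trap that drops when interacted with, trapping and damaging whatever it lands on.
; Interact enables physics; the first Hit freezes the cage and switches the side and top boxes to a player-blocking collision profile.
; It then teleports the first overlapping actor to TrapLocation on X and Z, keeping its Y, and calls GetHit if it is a BP_CharacterBase.
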(event `/Game/Blueprints/Interfaces/BPI_Interactable.Interact`
  (`PrimitiveComponent.SetSimulatePhysics` (`self.RenderComponent`) true))

(event `self.ReceiveHit`
  (params (MyComp :type "PrimitiveComponent Object Reference") (Other :type "Actor Object Reference") (OtherComp :type "PrimitiveComponent Object Reference") (bSelfMoved :type Boolean) (HitLocation :type "Vector Structure") (HitNormal :type "Vector Structure") (NormalImpulse :type "Vector Structure") (Hit :type "HitResult Structure (by ref)"))
  (bind (_returnvalue_x _returnvalue_y) (`KismetMathLibrary.BreakVector` (`self.K2_GetActorLocation` (`self.TrappedActor`))))
  (bind (_returnvalue_x_2 _returnvalue_y_2 _returnvalue_z) (`KismetMathLibrary.BreakVector` (`SceneComponent.K2_GetComponentLocation` (`self.TrapLocation`))))
  (bind _output (`|GetArrayItem` (`PrimitiveComponent.GetOverlappingActors` (`self.RenderComponent`) "/Script/Engine.Actor")))
  (if (not (`self.Triggered`))
    ;[0 0 0] Stop physics so the cage doesn't move anymore.
    (`PrimitiveComponent.SetSimulatePhysics` (`self.RenderComponent`) false)
    (set `self.Triggered` true)
    (`self.SetTriggeredCollisions`)
    (`/Engine/EditorBlueprintResources/StandardMacros.IsValid` _output
      (:`Is Valid`
        (bind _output_get (set `self.TrappedActor` _output))
        (`self.K2_SetActorLocation` _output_get (`KismetMathLibrary.MakeVector` _returnvalue_x_2 _returnvalue_y _returnvalue_z) false true)
        (bind _asbp_character_base (cast `/Game/Blueprints/Characters/BP_CharacterBase` _output_get))
        (`/Game/Blueprints/Characters/BP_CharacterBase.Get Hit` _asbp_character_base (`self.Damage`))))))

(fn `SetTriggeredCollisions`
  (`PrimitiveComponent.SetCollisionProfileName` (`self.Box_Left`) (`self.BlockPlayerCollisionProfile`) true)
  (`PrimitiveComponent.SetCollisionProfileName` (`self.Box_Right`) (`self.BlockPlayerCollisionProfile`) true)
  (`PrimitiveComponent.SetCollisionProfileName` (`self.Box_Top`) (`self.BlockPlayerCollisionProfile`) true))

(fn `UserConstructionScript`)