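; BP_EnemyPatrolBox is a trigger volume that hands the player to a group of associated enemy AI as their combat target.
; When an actor implementing BPI_Player begins overlapping, it sends SetCombatTargetMessage with that actor to every valid entry in PatrolActors.
; When that actor ends overlap, it sends the same message with no target, clearing combat for those AI.
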(event `self.ReceiveActorBeginOverlap`
  (params (OtherActor :type "Actor Object Reference"))
  ;[0.2062 0.3594 0.1542] When player overlaps with box, set combat target for all associated AI
  (if (`KismetSystemLibrary.DoesImplementInterface` OtherActor "/Game/Blueprints/Interfaces/BPI_Player.BPI_Player_C")
    (for _array_element (`self.PatrolActors`)
      (`/Engine/EditorBlueprintResources/StandardMacros.IsValid` _array_element
        (:`Is Valid`
          (message `/Game/Blueprints/Interfaces/BPI_Enemy.SetCombatTarget` _array_element OtherActor))))))

(event `self.ReceiveActorEndOverlap`
  (params (OtherActor :type "Actor Object Reference"))
  ;[1 0.5208 0.5605] When player stops overlap with box, clear all combat targets for associated AI
  (if (`KismetSystemLibrary.DoesImplementInterface` OtherActor "/Game/Blueprints/Interfaces/BPI_Player.BPI_Player_C")
    (for _array_element (`self.PatrolActors`)
      (`/Engine/EditorBlueprintResources/StandardMacros.IsValid` _array_element
        (:`Is Valid`
          (message `/Game/Blueprints/Interfaces/BPI_Enemy.SetCombatTarget` _array_element null))))))

(fn `UserConstructionScript`)