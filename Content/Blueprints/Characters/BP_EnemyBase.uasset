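; BP_EnemyBase is an enemy character base that connects combat events to its AI Blackboard and an overhead health bar.
; It writes alive, combat target and hit-reacting states to the Blackboard, plays attack animations and can turn around.
; GetHit updates the health bar and, only when that widget is valid, calls Die at zero health.
; Die clears the alive key, disables capsule collision, hides the bar and schedules destruction.
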(event `self.ReceiveBeginPlay`
  (`parent.ReceiveBeginPlay`)
  (bind _aswbp_enemy_health_bar (cast `/Game/Blueprints/UI/WBP_EnemyHealthBar` (`WidgetComponent.GetUserWidgetObject` (`self.HealthBarWidget`))))
  (set `self.EnemyHealthBar` _aswbp_enemy_health_bar)
  (`BlackboardComponent.SetValueAsBool` (`AIBlueprintHelperLibrary.GetBlackboard` (`self.GetController`)) (`self.AliveBBKeyName`) true))

(event `/Game/Blueprints/Interfaces/BPI_Enemy.SetCombatTarget`
  (params (CombatTarget :type "Actor Object Reference"))
  (`BlackboardComponent.SetValueAsObject` (`AIBlueprintHelperLibrary.GetBlackboard` (`self.GetController`)) (`self.CombatTargetBBKeyName`) CombatTarget))

(event `/Game/Blueprints/Interfaces/BPI_Enemy.Attack`
  (`self.PlayAttackAnim`))

(event `/Game/Blueprints/Interfaces/BPI_Enemy.SetHitReacting`
  (params (IsGettingHit :type Boolean))
  (`BlackboardComponent.SetValueAsBool` (`AIBlueprintHelperLibrary.GetBlackboard` (`self.GetController`)) (`self.GettingHitBBKeyName`) IsGettingHit))

(fn `ChangeDirection`
  (`self.K2_SetActorRotation` (`KismetMathLibrary.ComposeRotators` (`self.K2_GetActorRotation`) (struct :`Yaw` 180.0))))

(fn `Die`
  (`|ExecutionSequence`
    (:`then_0`
      ;[0.2703 0.3551 0.849] Disable Behavior Tree
      (`BlackboardComponent.SetValueAsBool` (`AIBlueprintHelperLibrary.GetBlackboard` (`self.GetController`)) (`self.AliveBBKeyName`) false))
    (:`then_1`
      ;[0.2703 0.3551 0.849] Disable Collision
      (`PrimitiveComponent.SetCollisionEnabled` (`self.CapsuleComponent`) "NoCollision"))
    (:`then_2`
      ;[0.2703 0.3551 0.849] Hide Health Bar
      (`SceneComponent.SetVisibility` (`self.HealthBarWidget`) false false))
    (:`then_3`
      ;[0.2703 0.3551 0.849] Destroy Actor After 5 Seconds
      (`self.SetLifeSpan` 5.0))))

(fn `Get Hit`
  (params (InDamage :type "Float (double-precision)"))
  (`parent.Get Hit` InDamage)
  (bind _enemyhealthbar (`self.EnemyHealthBar`)
    (:`then`
      (`/Game/Blueprints/UI/WBP_EnemyHealthBar.SetHealthPercent` _enemyhealthbar (`KismetMathLibrary.SafeDivide` (`self.Health`) (`self.MaxHealth`)))
      (if (<= (`self.Health`) 0.0)
        (`self.Die`)))
    (:`else`)))

(fn `UserConstructionScript`)